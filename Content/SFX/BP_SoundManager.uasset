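; BP_SoundManager switches the soundtrack according to the zone of the BP_Kite actor it finds at BeginPlay.
; Each Tick it polls the kite's zone and, on a change, picks one of four sounds for that zone.
; Two audio components alternate via a boolean flag, so the new sound fades in while the previous one fades out, giving an S-curve crossfade.
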(event EventTick
  (params (DeltaSeconds :type Float%20%28single-precision%29))
  (bind _kiteref (Variables|Default|GetKiteRef)
    (:then
      (bind _returnvalue (Default|GetZone _kiteref))
      (if (!= _returnvalue (Variables|Default|GetCurrentZone))
        (Variables|Default|SetCurrentZone _returnvalue)
        (Audio|Components|Audio|SetSound (CallFunction|GetAudio) (Utilities|Select :Index (Variables|Default|GetCurrentZone) :Option%200 "/Game/SFX/Isabel_1.Isabel_1" :Option%201 "/Game/SFX/Jurre.Jurre" :Option%202 "/Game/SFX/Vittu.Vittu" :Option%203 "/Game/SFX/Isabel_2.Isabel_2"))
        (Audio|Components|Audio|FadeOut (CallFunction|GetOldAudio) 3.0 0.0 "SCurve" :!class /Script/Engine.AudioComponent)
        (Audio|Components|Audio|FadeIn (CallFunction|GetAudio) 3.0 1.0 0.0 "SCurve" :!class /Script/Engine.AudioComponent)
        (Variables|Default|SetCurrentAudio (not (Variables|Default|GetCurrentAudio)))))
    (:else)))

(event EventBeginPlay
  (bind _returnvalue (Actor|GetActorOfClass "/Game/BIRDING/Kite/BP_Kite.BP_Kite_C"))
  (Variables|Default|SetKiteRef _returnvalue))

(fn ConstructionScript)

(fn GetAudio
  (return (select (Variables|Default|GetCurrentAudio) (Variables|Default|GetAudio1) (Variables|Default|GetAudio))))

(fn GetOldAudio
  (return (select (Variables|Default|GetCurrentAudio) (Variables|Default|GetAudio) (Variables|Default|GetAudio1))))