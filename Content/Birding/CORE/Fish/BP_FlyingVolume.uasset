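; BP_FlyingVolume is a box volume, hidden in game, that populates the air around the player's altitude with BP_Bird actors.
; Tick moves the box to the player's height, and construction sizes it from VolumeExtents.
; A looping timer spawns birds on its top or bottom face, favoring the top, while the box is high enough and ActiveBirds is below MaxBirds.
; Birds leaving the box are destroyed and decrement the count.
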(event OnComponentEndOverlap(Box)
  (params (OverlappedComponent :type Primitive%20Component%20Object%20Reference) (OtherActor :type Actor%20Object%20Reference) (OtherComp :type Primitive%20Component%20Object%20Reference) (OtherBodyIndex :type Integer))
  (bind _asbp_bird (Utilities|Casting|CastToBP_Bird OtherActor))
  (Actor|DestroyActor _asbp_bird)
  (Math|Integer|DecrementInt (Variables|Default|GetActiveBirds)))

(event EventBeginPlay
  (Utilities|FlowControl|Sequence
    (:then_0
      (Rendering|SetActorHiddenInGame true))
    (:then_1
      (Utilities|Time|SetTimerbyFunctionName 0 "SpawnBird" 1.0 true))))

(event EventTick
  (params (DeltaSeconds :type Float%20%28single-precision%29))
  (Transformation|SetWorldLocation (Variables|Default|GetBox) (Math|Vector|MakeVector 0.0 0.0 (.z (Transformation|GetActorLocation (Game|GetPlayerCharacter 0)))) true false))

(fn ConstructionScript
  (Components|Box|SetBoxExtent (Variables|Default|GetBox) (Variables|Settings|GetVolumeExtents) true))

(fn SpawnBird
  (bind _box (Variables|Default|GetBox))
  (bind _boxextent (Variables|/Script/Engine.BoxComponent|GetBoxExtent _box))
  (bind _returnvalue (* (.y _boxextent) 0.5))
  (if (and (> (.z (Transformation|GetWorldLocation _box)) 5e+02) (< (Variables|Default|GetActiveBirds) (Variables|Default|GetMaxBirds)))
    (Game|SpawnActorfromClass "/Game/Birding/CORE/Fish/BP_Bird.BP_Bird_C" (Math|Conversions|ToTransform(Vector) (+ (Transformation|GetWorldLocation _box) (Math|Vector|MakeVector 0.0 (Math|Random|RandomFloatinRange (* _returnvalue -1.0) _returnvalue) (* (.z _boxextent) (Math|Float|SelectFloat 1.0 -1.0 (Math|Random|RandomBoolwithWeight 0.7)))))) "Undefined" "MultiplyWithRoot" 0 0)
    (Math|Integer|IncrementInt (Variables|Default|GetActiveBirds))))