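; BP_Bird is a flying, flipbook-animated catchable creature, called a fish internally, that the player's kite captures for coins.
; On spawn it picks a random DT_Fishes row from the kite's current zone for speed, reward and visuals.
; Kite overlap hooks it and starts a capture timer scaled by pull strength and kite speed.
; Ending overlap beyond the capture distance frees it, and a looping timer restores its look; otherwise it awards coins and is destroyed.
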(event OnComponentEndOverlap(CollisionDetection)
  (params (OverlappedComponent :type Primitive%20Component%20Object%20Reference) (OtherActor :type Actor%20Object%20Reference) (OtherComp :type Primitive%20Component%20Object%20Reference) (OtherBodyIndex :type Integer))
  (bind _returnvalue (Transformation|GetActorLocation OtherActor))
  (bind _returnvalue_2 (Transformation|GetActorLocation))
  (bind _returnvalue_3 (- _returnvalue _returnvalue_2))
  (bind _returnvalue_4 (Math|Vector|VectorGetAbs _returnvalue_3))
  ;[1 1 1] Handle event where kite moves away from the fish
  (bind _returnvalue_5 (Actor|GetActorOfClass "/Game/Birding/CORE/Kite/BP_Kite.BP_Kite_C"))
  (if (== _returnvalue_5 OtherActor)
    (if (>= (+ (.x _returnvalue_4) (.y _returnvalue_4) (.z _returnvalue_4)) (+ (Variables|Default|GetFishCaptureZone) (Math|Float|MakeLiteralFloat 0.0)))
      (Variables|Default|SetIsFree? true))))

(event OnComponentBeginOverlap(CollisionDetection)
  (params (OverlappedComponent :type Primitive%20Component%20Object%20Reference) (OtherActor :type Actor%20Object%20Reference) (OtherComp :type Primitive%20Component%20Object%20Reference) (OtherBodyIndex :type Integer) (bFromSweep :type Boolean) (SweepResult :type Hit%20Result%20Structure%20%28by%20ref%29))
  ;[1 1 1] Detectiong Collision with a kite and processing catching phase
  (bind _returnvalue (Actor|GetActorOfClass "/Game/Birding/CORE/Kite/BP_Kite.BP_Kite_C"))
  (if (== _returnvalue OtherActor)
    (if (Variables|Default|GetIsFree?)
      (CallFunction|HandleBeingHooked))))

(event Custom|FreeFish
  ;[1 1 1] Free fish when kait moves away from it
  (if (Variables|Default|GetIsFree?)
    (Sprite|SetFlipbook (Variables|Default|GetPaperFlipbook) (.movementflipbook (Variables|Default|GetFishInfo)))
    (Sprite|SetSpriteColor (Variables|Default|GetPaperFlipbook) (Variables|Default|GetDefaultColor))))

(event Custom|FinishFishCapture
  ;[1 1 1] Handle event when fish is caught
  (if (not (Variables|Default|GetIsFree?))
    (Audio|PlaySoundatLocation "/Game/Birding/SFX/Collection_Sound_V5.Collection_Sound_V5" (Transformation|GetActorLocation) "0, 0, 0" 1.0 1.0 0.0 0 0 0 0)
    (Default|AddCoins (stale Custom|HandleBeingHooked _asbp_kite) (Variables|FishSettings|GetReward))
    (Actor|DestroyActor)))

(event Custom|HandleBeingHooked
  (bind _paperflipbook (Variables|Default|GetPaperFlipbook))
  ;[1 1 1] Event for when the fish got Hooked
  (Variables|Default|SetIsFree? false)
  (bind _returnvalue (Utilities|GetDataTableRow "/Game/Birding/CORE/Fish/DT_Fishes.DT_Fishes" (Variables|Default|GetFishName))
    (:then
      (Sprite|SetFlipbook _paperflipbook (.hookedflipbook _returnvalue))
      (Sprite|SetSpriteColor _paperflipbook (Variables|Default|GetColorOnCatching))
      (Utilities|Time|SetTimerbyEvent (delegate Custom|FreeFish) 0.1 true)
      ;[1 1 1] Determine time that kite have to be around fish to catch it
      (bind _asbp_kite (Utilities|Casting|CastToBP_Kite (Game|Player|GetPlayerPawn 0)))
      (Utilities|Time|SetTimerbyEvent (delegate Custom|FinishFishCapture) (/ (.pullstrength (Variables|Default|GetFishInfo)) (/ (Variables|/Game/Birding/CORE/Kite/BP_Kite.BP_Kite_C|GetKiteFlyingSpeed _asbp_kite) (Math|Float|MakeLiteralFloat 2e+02)))))))

(event EventBeginPlay
  (Pawn|Components|CharacterMovement|SetMovementMode (Variables|Character|GetCharacterMovement) "MOVE_Flying" 0)
  (CallFunction|SetFishType))

(fn ConstructionScript
  (Sprite|SetSpriteColor (Variables|Default|GetPaperFlipbook) (Variables|Default|GetDefaultColor)))

(fn SetFishType
  (bind _asbp_kite (Utilities|Casting|CastToBP_Kite (Game|GetPlayerCharacter 0)))
  (bind _returnvalue (Default|GetZone _asbp_kite))
  (bind _output_get (Variables|Default|SetFishName (Utilities|Select :Index (Utilities|Select :Index _returnvalue :Option%200 (Math|Random|RandomIntegerinRange 0 2) :Option%201 (Math|Random|RandomIntegerinRange 3 6) :Option%202 (Math|Random|RandomIntegerinRange 7 10)) :Option%200 "FishA" :Option%201 "FishB" :Option%202 "FishC" :Option%203 "FishD" :Option%204 "FishE" :Option%205 "FishF" :Option%206 "FishG" :Option%207 "FishH" :Option%208 "FishI" :Option%209 "FishJ" :Option%2010 "FishK")))
  (bind _returnvalue_2 (Utilities|GetDataTableRow "/Game/Birding/CORE/Fish/DT_Fishes.DT_Fishes" _output_get)
    (:then
      (bind _output_get_2 (Variables|Default|SetFishInfo _returnvalue_2))
      (Variables|FishSettings|SetSpeed (.speed _output_get_2))
      (Variables|FishSettings|SetReward (.rewardwhencaught _output_get_2))
      (Sprite|SetFlipbook (Variables|Default|GetPaperFlipbook) (.movementflipbook _output_get_2)))))