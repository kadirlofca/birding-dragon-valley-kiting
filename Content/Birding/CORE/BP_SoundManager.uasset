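; BP_SoundManager is an actor that switches music tracks as the BP_Kite moves between zones.
; Each Tick polls the kite's zone; a change selects that zone's track and crossfades two audio components over three seconds, then flips their roles.
; In zones 1 and 2, fractional zone progress progressively lowers pitch on GetAudio's component, which after the flip is the one that faded out.
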(event EventTick
  (params (DeltaSeconds :type Float%20%28single-precision%29))
  (bind _audio (CallFunction|GetAudio))
  (Utilities|FlowControl|Sequence
    (:then_0
      (bind _kiteref (Variables|Default|GetKiteRef)
        (:then
          (bind _returnvalue (Default|GetZone _kiteref))
          (if (!= _returnvalue (Variables|Default|GetCurrentZone))
            (Variables|Default|SetCurrentZone _returnvalue)
            (Audio|Components|Audio|SetSound (CallFunction|GetAudio) (Utilities|Select :Index (Variables|Default|GetCurrentZone) :Option%200 "/Game/Birding/SFX/Isabel_1.Isabel_1" :Option%201 "/Game/Birding/SFX/Jurre_van_den_Berg_-_Birding_Sky_v1_1.Jurre_van_den_Berg_-_Birding_Sky_v1_1" :Option%202 "/Game/Birding/SFX/Vittu.Vittu" :Option%203 "/Game/Birding/SFX/Isabel_2.Isabel_2" :Option%204 "/Game/Birding/SFX/Jurre_van_den_Berg_-_Birding_Galaxy_v1_1.Jurre_van_den_Berg_-_Birding_Galaxy_v1_1"))
            (Audio|Components|Audio|FadeOut (CallFunction|GetOldAudio) 3.0 0.0 "SCurve" :!class /Script/Engine.AudioComponent)
            (Audio|Components|Audio|FadeIn (CallFunction|GetAudio) 3.0 1.0 0.0 "SCurve" :!class /Script/Engine.AudioComponent)
            (Variables|Default|SetCurrentAudio (not (Variables|Default|GetCurrentAudio)))))
        (:else)))
    (:then_1
      (bind (_returnvalue_2 _raw) (Default|GetZone _kiteref))
      (if (== _returnvalue_2 1)
        (Audio|Components|Audio|SetPitchMultiplier _audio (Math|Float|MapRangeClamped (Math|Float|%(Float) _raw 1.0) 0.0 1.0 1.0 0.933))
        (elif (== _returnvalue_2 2)
          (Audio|Components|Audio|SetPitchMultiplier _audio (Math|Float|MapRangeClamped (Math|Float|%(Float) _raw 1.0) 0.0 1.0 0.933 0.8)))))))

(event EventBeginPlay
  (bind _returnvalue (Actor|GetActorOfClass "/Game/Birding/Core/Kite/BP_Kite.BP_Kite_C"))
  (Variables|Default|SetKiteRef _returnvalue))

(fn ConstructionScript)

(fn GetAudio
  (return (select (Variables|Default|GetCurrentAudio) (Variables|Default|GetAudio1) (Variables|Default|GetAudio))))

(fn GetOldAudio
  (return (select (Variables|Default|GetCurrentAudio) (Variables|Default|GetAudio) (Variables|Default|GetAudio1))))