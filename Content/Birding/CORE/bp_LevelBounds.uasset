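; Level bounds actor that keeps the player's BP_Kite within a horizontal corridor of a set Width, centred on world Y zero.
; On BeginPlay it caches the first BP_Kite found in the level.
; Each Tick, a kite beyond half the Width gets movement input back toward the centre, scaled by OutOfBoundsWindPower, as a soft wall.
; A looping one-second timer redraws tall red debug lines at both edges.
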(event EventBeginPlay
  (Utilities|FlowControl|Sequence
    (:then_0
      (CallFunction|Debug))
    (:then_1
      (Utilities|Time|SetTimerbyFunctionName 0 "Debug" 1.0 true))
    (:then_2
      (bind _returnvalue (Actor|GetActorOfClass "/Game/Birding/CORE/Kite/BP_Kite.BP_Kite_C"))
      (Variables|Default|SetKite _returnvalue))))

(event EventTick
  (params (DeltaSeconds :type Float%20%28single-precision%29))
  (bind _kite (Variables|Default|GetKite))
  (bind _returnvalue (Transformation|GetActorLocation _kite))
  (Variables|Default|GetKite
    (:then
      (if (> (Math|Float|Absolute(Float) (.y _returnvalue)) (/ (Variables|Default|GetWidth) 2.0))
        (bind _asbp_kite (Utilities|Casting|CastToBP_Kite (Variables|Default|GetKite)))
        (Pawn|Input|AddMovementInput _asbp_kite (Math|Vector|MakeVector 0.0 (* (Math|Float|Sign(Float) (.y _returnvalue)) (Variables|Default|GetOutOfBoundsWindPower) -1.0) 0.0) 1.0 false)))
    (:else)))

(fn ConstructionScript)

(fn Debug
  (bind _width (Variables|Default|GetWidth))
  (bind _returnvalue (* _width 0.5))
  (bind _returnvalue_2 (* _width -0.5))
  (Rendering|Debug|DrawDebugLine (Math|Vector|MakeVector 0.0 _returnvalue_2 0.0) (Math|Vector|MakeVector 0.0 _returnvalue_2 99999.0) "(R=1.000000,G=0.000000,B=0.006919,A=1.000000)" 1.0 1e+01)
  (Rendering|Debug|DrawDebugLine (Math|Vector|MakeVector 0.0 _returnvalue 0.0) (Math|Vector|MakeVector 0.0 _returnvalue 99999.0) "(R=1.000000,G=0.000000,B=0.006919,A=1.000000)" 1.0 1e+01))