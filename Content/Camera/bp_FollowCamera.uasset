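; Follow camera actor that tracks a settable CameraTarget from a fixed distance along negative X.
; Each tick, while the target is valid, it eases the camera toward the target's Y and Z, clamping Y symmetrically to CameraMaxY.
; It then smoothly rotates the camera to look at the target, with separate interpolation speeds for movement and rotation.
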(event EventTick
  (params (DeltaSeconds :type Float%20%28single-precision%29))
  (Variables|Default|GetCameraTarget
    (:then
      (CallFunction|UpdateCameraLocation)
      (CallFunction|UpdateCameraRotation))
    (:else)))

(fn ConstructionScript)

(fn UpdateCameraLocation
  (bind _returnvalue (Utilities|Time|GetWorldDeltaSeconds))
  (bind _camera (Variables|Default|GetCamera))
  (bind _cameratarget (Variables|Default|GetCameraTarget))
  (bind _cameramovespeed (Variables|Default|GetCameraMoveSpeed))
  (bind _returnvalue_2 (Transformation|GetWorldLocation _camera))
  (bind _returnvalue_3 (Transformation|GetActorLocation _cameratarget))
  (bind _returnvalue_4 (Math|Vector|MakeVector 0.0 (.y _returnvalue_3) (.z _returnvalue_3)))
  (bind _returnvalue_5 (Math|Interpolation|VInterpTo _returnvalue_2 _returnvalue_4 _returnvalue _cameramovespeed))
  (Transformation|SetWorldLocation (Variables|Default|GetCamera) (Math|Vector|MakeVector (* (Variables|Default|GetCameraDistance) -1.0) (* (Math|Float|Sign(Float) (.y _returnvalue_5)) (Math|Float|Min(Float) (Math|Float|Absolute(Float) (.y _returnvalue_5)) (Variables|Default|GetCameraMaxY))) (.z _returnvalue_5)) false false))

(fn UpdateCameraRotation
  (Transformation|SetWorldRotation (Variables|Default|GetCamera) (Math|Interpolation|RInterpTo (Transformation|GetWorldRotation (Variables|Default|GetCamera)) (Math|Rotator|FindLookatRotation (Transformation|GetWorldLocation (Variables|Default|GetCamera)) (Transformation|GetActorLocation (Variables|Default|GetCameraTarget))) (Utilities|Time|GetWorldDeltaSeconds) (Variables|Default|GetCameraRotateSpeed)) false false))

(fn SetCameraTarget
  (params (CameraTarget :type Actor%20Object%20Reference))
  (Variables|Default|SetCameraTarget CameraTarget))