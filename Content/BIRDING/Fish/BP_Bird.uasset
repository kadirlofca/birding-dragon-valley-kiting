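; Flying 2D catchable creature (a "fish" in code, despite the bird name) that the player's kite hooks on contact.
; On BeginPlay it picks a random type from the range for the kite's current zone and loads speed, reward and flipbook from DT_Fishes.
; Kite overlap plays a sound and swaps to a darkened hooked flipbook, then destroys it after a delay scaled by pull strength over kite speed.
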(event OnComponentBeginOverlap(CollisionDetection)
  (params (OverlappedComponent :type Primitive%20Component%20Object%20Reference) (OtherActor :type Actor%20Object%20Reference) (OtherComp :type Primitive%20Component%20Object%20Reference) (OtherBodyIndex :type Integer) (bFromSweep :type Boolean) (SweepResult :type Hit%20Result%20Structure%20%28by%20ref%29))
  ;[1 1 1] Detectiong Collision with a kite and processing catching phase
  (bind _returnvalue (Actor|GetActorOfClass "/Game/BIRDING/Kite/BP_Kite.BP_Kite_C"))
  (if (== _returnvalue OtherActor)
    (if (Variables|Default|GetIsFree?)
      (Audio|PlaySoundatLocation "/Game/SFX/Collection_Sound_V5.Collection_Sound_V5" (Transformation|GetActorLocation) "0, 0, 0" 1.0 1.0 0.0 0 0 0 0)
      (CallFunction|HandleBeingHooked))))

(event Custom|HandleBeingHooked
  (bind _paperflipbook (Variables|Default|GetPaperFlipbook))
  ;[1 1 1] Event for when the fish got Hooked
  (Variables|Default|SetIsFree? false)
  (bind _returnvalue (Utilities|GetDataTableRow "/Game/BIRDING/Fish/DT_Fishes.DT_Fishes" (Variables|Default|GetFishName))
    (:then
      (Sprite|SetFlipbook _paperflipbook (.hookedflipbook _returnvalue))
      (Sprite|SetSpriteColor _paperflipbook "(R=0.197917,G=0.197917,B=0.197917,A=1.000000)")
      ;;[1 1 1] Adjust animation playback based on the kite speed (and fish strength)
      (bind _asbp_kite (Utilities|Casting|CastToBP_Kite (Game|Player|GetPlayerPawn 0)))
      (Utilities|FlowControl|Delay (/ (.pullstrength _returnvalue) (/ (Variables|/Game/BIRDING/Kite/BP_Kite.BP_Kite_C|GetKiteFlyingSpeed _asbp_kite) 2e+02)))
      (Actor|DestroyActor))))

(event EventBeginPlay
  (Pawn|Components|CharacterMovement|SetMovementMode (Variables|Character|GetCharacterMovement) "MOVE_Flying" 0)
  (CallFunction|SetFishType))

(fn ConstructionScript)

(fn SetFishType
  (bind _asbp_kite (Utilities|Casting|CastToBP_Kite (Game|GetPlayerCharacter 0)))
  (bind _returnvalue (Default|GetZone _asbp_kite))
  (bind _output_get (Variables|Default|SetFishName (Utilities|Select :Index (Utilities|Select :Index _returnvalue :Option%200 (Math|Random|RandomIntegerinRange 0 2) :Option%201 (Math|Random|RandomIntegerinRange 3 6) :Option%202 (Math|Random|RandomIntegerinRange 7 10)) :Option%200 "FishA" :Option%201 "FishB" :Option%202 "FishC" :Option%203 "FishD" :Option%204 "FishE" :Option%205 "FishF" :Option%206 "FishG" :Option%207 "FishH" :Option%208 "FishI" :Option%209 "FishJ" :Option%2010 "FishK")))
  (bind _returnvalue_2 (Utilities|GetDataTableRow "/Game/BIRDING/Fish/DT_Fishes.DT_Fishes" _output_get)
    (:then
      (Variables|FishSettings|SetSpeed (.speed _returnvalue_2))
      (Variables|FishSettings|SetReward (.value _returnvalue_2))
      (Sprite|SetFlipbook (Variables|Default|GetPaperFlipbook) (.movementflipbook _returnvalue_2)))))