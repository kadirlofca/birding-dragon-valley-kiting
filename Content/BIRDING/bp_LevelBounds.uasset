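; Level bounds actor for the kite game that keeps BP_Kite within a horizontal play width along world Y.
; BeginPlay draws red debug lines at both width edges, positions the left and right border boxes just inside them, and finds the kite.
; Each tick, once the kite strays over a quarter of the width from Y zero, constant-strength "wind" movement input pushes it back toward center.
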(event EventBeginPlay
  (Utilities|FlowControl|Sequence
    (:then_0
      (CallFunction|Debug))
    (:then_1
      (CallFunction|SetBorderLocation))
    (:then_2
      (bind _returnvalue (Actor|GetActorOfClass "/Game/BIRDING/Kite/BP_Kite.BP_Kite_C"))
      (Variables|Default|SetKite _returnvalue))))

(event EventTick
  (params (DeltaSeconds :type Float%20%28single-precision%29))
  (bind _kite (Variables|Default|GetKite))
  (bind _returnvalue (Transformation|GetActorLocation _kite))
  (Variables|Default|GetKite
    (:then
      (if (> (Math|Float|Absolute(Float) (.y _returnvalue)) (/ (Variables|Default|GetWidth) 4.0))
        (bind _asbp_kite (Utilities|Casting|CastToBP_Kite (Variables|Default|GetKite)))
        (Pawn|Input|AddMovementInput _asbp_kite (Math|Vector|MakeVector 0.0 (* (Math|Float|Sign(Float) (.y _returnvalue)) (Variables|Default|GetOutOfBoundsWindPower) -1.0) 0.0) 1.0 false)))
    (:else)))

(fn ConstructionScript)

(fn Debug
  (bind _width (Variables|Default|GetWidth))
  (Rendering|Debug|DrawDebugLine (Math|Vector|MakeVector 0.0 (* _width -0.5) -99999.0) (Math|Vector|MakeVector 0.0 0.0 99999.0) "(R=1.000000,G=0.000000,B=0.006919,A=1.000000)" 9999999.0 1e+01)
  (Rendering|Debug|DrawDebugLine (Math|Vector|MakeVector 0.0 (* _width 0.5) -99999.0) (Math|Vector|MakeVector 0.0 0.0 99999.0) "(R=1.000000,G=0.000000,B=0.006919,A=1.000000)" 9999999.0 1e+01))

(fn SetBorderLocation
  (bind _width (Variables|Default|GetWidth))
  (bind _rightborder (Variables|Default|GetRightBorder))
  (bind _returnvalue (/ _width 2.0))
  (bind _boxextent (Variables|/Script/Engine.BoxComponent|GetBoxExtent _rightborder))
  (bind _returnvalue_2 (* (.y _boxextent) 2.0))
  (bind _returnvalue_3 (- _returnvalue _returnvalue_2))
  (Transformation|SetWorldLocation (Variables|Default|GetLeftBorder) (Math|Vector|MakeVector 0.0 _returnvalue_3 0.0) false false)
  (Transformation|SetWorldLocation (Variables|Default|GetRightBorder) (Math|Vector|MakeVector 0.0 (* _returnvalue_3 -1.0) 0.0) false false))